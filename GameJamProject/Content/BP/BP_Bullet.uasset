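; BP_Bullet is a projectile actor that flies in a set direction and expires after four seconds.
; Tick moves it by a swept local offset built from its For vector and Speed.
; Sphere1 overlaps with actors tagged "hit" spawn a pooled Niagara explosion and destroy the bullet.
; Those actors are destroyed too if they also carry the "die" tag.
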(event `self.ReceiveBeginPlay`
  (`KismetSystemLibrary.Delay` 4.0)
  (`self.K2_DestroyActor`))

(event `self.ReceiveTick`
  (params (DeltaSeconds :type "Float (single-precision)"))
  (`self.K2_AddActorLocalOffset` (* (`self.For`) (* (`self.Speed`) DeltaSeconds)) true))

(event `self.Sphere1.OnComponentBeginOverlap`
  (params (OverlappedComponent :type "PrimitiveComponent Object Reference") (OtherActor :type "Actor Object Reference") (OtherComp :type "PrimitiveComponent Object Reference") (OtherBodyIndex :type Integer) (bFromSweep :type Boolean) (SweepResult :type "HitResult Structure (by ref)"))
  (if (`self.ActorHasTag` OtherActor "hit")
    (`NiagaraFunctionLibrary.SpawnSystemAtLocation` "/Game/VFX/ParticleSystems/NS_Explosion.NS_Explosion" (`self.K2_GetActorLocation`) (struct) (1.0 1.0 1.0) true true "AutoRelease")
    (if (`self.ActorHasTag` OtherActor "die")
      (`self.K2_DestroyActor` OtherActor))
    (`self.K2_DestroyActor`)))

(fn `UserConstructionScript`)